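; BP_Object is a collectible item that reports its Type to BP_GS_GameState through CatchItem when a BP_Character overlaps its mesh, then destroys itself.
; The construction script uses Type as a row index into the BP_ObjectList data table to set the item material and a beam material on a second mesh.
; On BeginPlay, a timeline moves the main mesh vertically around its initial location.
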(event OnComponentBeginOverlap(Mesh)
  (params (OverlappedComponent :type Primitive%20Component%20Object%20Reference) (OtherActor :type Actor%20Object%20Reference) (OtherComp :type Primitive%20Component%20Object%20Reference) (OtherBodyIndex :type Integer) (bFromSweep :type Boolean) (SweepResult :type Hit%20Result%20Structure%20%28by%20ref%29))
  (Utilities|Casting|CastToBP_Character OtherActor)
  (bind _asbp_gs_game_state (Utilities|Casting|CastToBP_GS_GameState (Game|GetGameState)))
  (Default|CatchItem _asbp_gs_game_state (Variables|Default|GetType))
  (Actor|DestroyActor))

(event EventBeginPlay
  (Variables|Default|SetInitialLocation (Variables|/Script/Engine.SceneComponent|GetRelativeLocation (Variables|Default|GetMesh)))
  (bind _height (Timeline|ChangeHeight PlayFromStart)
    (:Update
      (Transformation|SetRelativeLocation (Variables|Default|GetMesh) (Math|Vector|MakeVector (.x (Variables|Default|GetInitialLocation)) (.y (Variables|Default|GetInitialLocation)) (+ (.z (Variables|Default|GetInitialLocation)) _height)) false false))))

(fn ConstructionScript
  (CallFunction|UpdateMaterial))

(fn UpdateMaterial
  (bind _type (Variables|Default|GetType))
  (bind _returnvalue (Math|Conversions|ToInteger(Byte) _type))
  (bind _outrownames (DataTable|GetDataTableRowNames "/Game/objects/BP_ObjectList.BP_ObjectList"))
  (if (< _returnvalue (Utilities|Array|Length _outrownames))
    (bind _returnvalue_2 (Utilities|GetDataTableRow "/Game/objects/BP_ObjectList.BP_ObjectList" (Utilities|Array|Get(acopy) _outrownames _returnvalue))
      (:then
        (Rendering|Material|SetMaterial (Variables|Default|GetMesh) 0 (.Material (Utilities|Struct|BreakBP_ObjectInfos _returnvalue_2)))
        (Rendering|Material|SetMaterial (Variables|Default|GetStaticMesh) 0 (.BeamMat (Utilities|Struct|BreakBP_ObjectInfos _returnvalue_2)))))))