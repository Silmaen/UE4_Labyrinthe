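; BP_FootSteps plays alternating left and right footstep sounds as distance accumulates.
; UpdateDistance adds each supplied distance to a running total and, once it exceeds the step length, subtracts one step and flips the foot.
; The cues play at the world origin rather than at a character's position.
; BeginPlay caches BP_GS_GameState, though this graph never reads it, and Tick is disabled.
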(event Custom|UpdateDistance
  (params (Distance :type Float%20%28single-precision%29))
  (bind _stepdistance (Variables|Default|GetStepDistance))
  (bind _output_get (Variables|Default|SetcurDistance (+ Distance (Variables|Default|GetcurDistance))))
  (if (> _output_get _stepdistance)
    (Variables|Default|SetcurDistance (- (Variables|Default|GetcurDistance) _stepdistance))
    (if (Variables|Default|Getleft)
      (Variables|Default|Setleft false)
      (Audio|PlaySoundatLocation "/Game/Sound/footsteps/footstep_left1_Cue.footstep_left1_Cue" "0, 0, 0" "0, 0, 0" 1.0 1.0 0.0 0 0 0)
      (else
        (Variables|Default|Setleft true)
        (Audio|PlaySoundatLocation "/Game/Sound/footsteps/footstep_right1_Cue.footstep_right1_Cue" "0, 0, 0" "0, 0, 0" 1.0 1.0 0.0 0 0 0)))))

(event EventBeginPlay
  (bind _asbp_gs_game_state (Utilities|Casting|CastToBP_GS_GameState (Game|GetGameState)))
  (Variables|Default|SetGameState _asbp_gs_game_state))

(event EventTick
  (params (DeltaSeconds :type Float%20%28single-precision%29)))