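; BP_Tile is a maze-style tile actor with ground and walls, configured entirely in the construction script by layout Type and EffectType.
; Type selects the wall mesh, from four-way junction to dead end.
; It then creates dynamic material instances for ground, walls and wall tops.
; EffectType comparisons become scalar parameters on all three, switching between labyrinth, fire, leaf, ice and crystal looks without separate materials per theme.
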(event EventBeginPlay)

(event Collision|EventActorBeginOverlap
  (params (OtherActor :type Actor%20Object%20Reference)))

(event EventTick
  (params (DeltaSeconds :type Float%20%28single-precision%29)))

(fn ConstructionScript
  (CallFunction|SetTileType)
  (CallFunction|CreateDynamicMaterials)
  (CallFunction|SetTileMaterial))

(fn SetTileType
  (bind _walls (Variables|Default|GetWalls))
  (switch Utilities|FlowControl|Switch|SwitchonE_TileType (Variables|TileParameter|GetType)
    (:NewEnumerator0
      (Components|StaticMesh|SetStaticMesh _walls "/Game/Tiles/4-ways.4-ways"))
    (:NewEnumerator1
      (Components|StaticMesh|SetStaticMesh _walls "/Game/Tiles/3-ways.3-ways"))
    (:NewEnumerator2
      (Components|StaticMesh|SetStaticMesh _walls "/Game/Tiles/2-ways.2-ways"))
    (:NewEnumerator3
      (Components|StaticMesh|SetStaticMesh _walls "/Game/Tiles/1-way.1-way"))))

(fn CreateDynamicMaterials
  (bind _walls (Variables|Default|GetWalls))
  (bind _returnvalue (Rendering|Material|CreateDynamicMaterialInstance "/Game/Tiles/M_Ground.M_Ground" "None" :!class /Script/Engine.KismetMaterialLibrary))
  (bind _output_get (Variables|Materials|SetGroundMaterial _returnvalue))
  (Rendering|Material|SetMaterial (Variables|Default|GetGround) 0 _output_get)
  (bind _returnvalue_2 (Rendering|Material|CreateDynamicMaterialInstance "/Game/Tiles/M_Walls.M_Walls" "None" :!class /Script/Engine.KismetMaterialLibrary))
  (bind _output_get_2 (Variables|Materials|SetWallMaterial _returnvalue_2))
  (Rendering|Material|SetMaterial _walls 0 _output_get_2)
  (bind _returnvalue_3 (Rendering|Material|CreateDynamicMaterialInstance "/Game/Tiles/M_TopWall.M_TopWall" "None" :!class /Script/Engine.KismetMaterialLibrary))
  (bind _output_get_3 (Variables|Materials|SetTopWallMaterial _returnvalue_3))
  (Rendering|Material|SetMaterial _walls 1 _output_get_3))

(fn SetTileMaterial
  (bind _effecttype (Variables|TileParameter|GetEffectType))
  (bind _wallmaterial (Variables|Materials|GetWallMaterial))
  (bind _topwallmaterial (Variables|Materials|GetTopWallMaterial))
  (bind _groundmaterial (Variables|Materials|GetGroundMaterial))
  (bind _effecttype_2 (Variables|TileParameter|GetEffectType))
  (bind _effecttype_3 (Variables|TileParameter|GetEffectType))
  (Utilities|FlowControl|Sequence
    (:then_0
      (Rendering|Material|SetScalarParameterValue _groundmaterial "Laby" (Math|Conversions|ToFloat(Boolean) (Utilities|Enum|Equal(Enum) _effecttype_2 "NewEnumerator5")) :!class /Script/Engine.MaterialInstanceDynamic)
      (Rendering|Material|SetScalarParameterValue _groundmaterial "Fire" (Math|Conversions|ToFloat(Boolean) (Utilities|Enum|Equal(Enum) _effecttype_2 "NewEnumerator1")) :!class /Script/Engine.MaterialInstanceDynamic)
      (Rendering|Material|SetScalarParameterValue _groundmaterial "Feuille" (Math|Conversions|ToFloat(Boolean) (Utilities|Enum|Equal(Enum) _effecttype_2 "NewEnumerator2")) :!class /Script/Engine.MaterialInstanceDynamic)
      (Rendering|Material|SetScalarParameterValue _groundmaterial "Glace" (Math|Conversions|ToFloat(Boolean) (Utilities|Enum|Equal(Enum) _effecttype_2 "NewEnumerator3")) :!class /Script/Engine.MaterialInstanceDynamic)
      (Rendering|Material|SetScalarParameterValue _groundmaterial "Crystal" (Math|Conversions|ToFloat(Boolean) (Utilities|Enum|Equal(Enum) _effecttype_2 "NewEnumerator4")) :!class /Script/Engine.MaterialInstanceDynamic))
    (:then_1
      (Rendering|Material|SetScalarParameterValue _wallmaterial "Laby" (Math|Conversions|ToFloat(Boolean) (Utilities|Enum|Equal(Enum) _effecttype_3 "NewEnumerator5")) :!class /Script/Engine.MaterialInstanceDynamic)
      (Rendering|Material|SetScalarParameterValue _wallmaterial "Fire" (Math|Conversions|ToFloat(Boolean) (Utilities|Enum|Equal(Enum) _effecttype_3 "NewEnumerator1")) :!class /Script/Engine.MaterialInstanceDynamic)
      (Rendering|Material|SetScalarParameterValue _wallmaterial "Feuille" (Math|Conversions|ToFloat(Boolean) (Utilities|Enum|Equal(Enum) _effecttype_3 "NewEnumerator2")) :!class /Script/Engine.MaterialInstanceDynamic)
      (Rendering|Material|SetScalarParameterValue _wallmaterial "Glace" (Math|Conversions|ToFloat(Boolean) (Utilities|Enum|Equal(Enum) _effecttype_3 "NewEnumerator3")) :!class /Script/Engine.MaterialInstanceDynamic)
      (Rendering|Material|SetScalarParameterValue _wallmaterial "Crystal" (Math|Conversions|ToFloat(Boolean) (Utilities|Enum|Equal(Enum) _effecttype_3 "NewEnumerator4")) :!class /Script/Engine.MaterialInstanceDynamic))
    (:then_2
      (Rendering|Material|SetScalarParameterValue _topwallmaterial "Laby" (Math|Conversions|ToFloat(Boolean) (Utilities|Enum|Equal(Enum) _effecttype "NewEnumerator5")) :!class /Script/Engine.MaterialInstanceDynamic)
      (Rendering|Material|SetScalarParameterValue _topwallmaterial "Fire" (Math|Conversions|ToFloat(Boolean) (Utilities|Enum|Equal(Enum) _effecttype "NewEnumerator1")) :!class /Script/Engine.MaterialInstanceDynamic)
      (Rendering|Material|SetScalarParameterValue _topwallmaterial "Feuille" (Math|Conversions|ToFloat(Boolean) (Utilities|Enum|Equal(Enum) _effecttype "NewEnumerator2")) :!class /Script/Engine.MaterialInstanceDynamic)
      (Rendering|Material|SetScalarParameterValue _topwallmaterial "Glace" (Math|Conversions|ToFloat(Boolean) (Utilities|Enum|Equal(Enum) _effecttype "NewEnumerator3")) :!class /Script/Engine.MaterialInstanceDynamic)
      (Rendering|Material|SetScalarParameterValue _topwallmaterial "Crystal" (Math|Conversions|ToFloat(Boolean) (Utilities|Enum|Equal(Enum) _effecttype "NewEnumerator4")) :!class /Script/Engine.MaterialInstanceDynamic))))