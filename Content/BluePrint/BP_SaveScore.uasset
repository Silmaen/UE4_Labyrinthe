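; BP_SaveScore maintains a high-score table of player name, level and time in seconds.
; AddScore appends a new entry, then calls SortTruncateArray to rebuild the list.
; That function uses a selection sort, repeatedly moving the best entry into Temp, keeping at most ten.
; An entry ranks better on higher level or otherwise shorter time, even if its level is lower.
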(fn SortTruncateArray
  (while (> (Utilities|Array|Length (Variables|Default|GetPlayerScores)) 0)
    (bind _output_get (LocalVariables|Setilowes 0))
    (LocalVariables|Settemplowest (Utilities|Array|Get(acopy) (Variables|Default|GetPlayerScores) _output_get))
    (for (_array_element _array_index) (Variables|Default|GetPlayerScores)
      (if (> (.level _array_element) (.level (LocalVariables|Gettemplowest)))
        (bind _output_get_2 (LocalVariables|Setilowes _array_index :!label _label))
        (LocalVariables|Settemplowest (Utilities|Array|Get(acopy) (Variables|Default|GetPlayerScores) _output_get_2))
        (elif (< (.timesecond _array_element) (.timesecond (LocalVariables|Gettemplowest)))
          (goto _label))))
    (if (< (Utilities|Array|Length (LocalVariables|Gettemp)) 10)
      (Utilities|Array|Add (LocalVariables|Gettemp) (LocalVariables|Gettemplowest)))
    (Utilities|Array|RemoveIndex (Variables|Default|GetPlayerScores) (LocalVariables|Getilowes)))
  (Variables|Default|SetPlayerScores (LocalVariables|Gettemp)))

(fn AddScore
  (params (PlayerName :type String) (Level :type Integer) (TimeSecond :type Float%20%28single-precision%29))
  (Utilities|Array|Add (Variables|Default|GetPlayerScores) (Utilities|Struct|MakeE_Score PlayerName Level TimeSecond))
  (CallFunction|SortTruncateArray))