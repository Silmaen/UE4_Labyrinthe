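; Game state that runs a timed item-collection level, tracking level and total time with a pausable chrono.
; NewLevel resets timer and items, then places the player and randomly typed BP_Object pickups on shuffled TargetPoints.
; Each CatchItem re-skins every BP_Tile and changes player speed, turning or braking by item type.
; The last item instead pauses the chrono and passes level time to BP_GameInstance to advance levels.
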(event Custom|NewGame
  (bind _gi (CallFunction|GetGameInstance))
  (Default|NewGame _gi)
  (Variables|Default|SetTotalTimeSeconds 0.0)
  (Variables|Default|SetLevelTime 0.0)
  (Variables|Default|Setpause? false)
  (bind _output_get (Variables|MapAttributes|SetCurrentLevel 0))
  (Game|OpenLevel(byName) (Utilities|Array|Get(acopy) (Variables|/Game/BluePrint/BP_GameInstance.BP_GameInstance_C|GetLevelsName _gi) _output_get)))

(event EventBeginPlay
  (CallFunction|GetGameInstance))

(event EventTick
  (params (DeltaSeconds :type Float%20%28single-precision%29))
  (if (not (Variables|Default|Getpause?))
    (Variables|Default|SetLevelTime (+ (Variables|Default|GetLevelTime) DeltaSeconds))
    (Variables|Default|SetTotalTimeSeconds (+ DeltaSeconds (Variables|Default|GetTotalTimeSeconds)))))

(fn ConstructionScript)

(fn GetTotalTime
  (return (Variables|Default|GetTotalTimeSeconds)))

(fn GetLevelTime
  (return (Variables|Default|GetLevelTime)))

(fn PauseChrono
  (Variables|Default|Setpause? true))

(fn ResumeChrono
  (Variables|Default|Setpause? false))

(fn ResetItems
  (params (NbItems :type Integer))
  (Variables|Default|SetNObjectInLevel NbItems)
  (Utilities|Array|Clear (Variables|Default|GetObjectsGathered)))

(fn NewLevel
  (params (LevelNbObjet :type Integer))
  (bind _gi (CallFunction|GetGameInstance))
  (Variables|Default|SetLevelTime 0.0)
  (Variables|Default|Setpause? true)
  (Variables|Default|SetTotalTimeSeconds (Default|GetTotalTime _gi))
  (Items|ResetItems LevelNbObjet)
  (Levels|PlacePlayerandObjects))

(fn CatchItem
  (params (ItemGathered :type BP_ObjectTypes%20Enum%20%28by%20ref%29 :default "NewEnumerator0"))
  (bind _objectsgathered (Variables|Default|GetObjectsGathered))
  (Utilities|Array|Add _objectsgathered ItemGathered)
  (if (>= (Utilities|Array|Length _objectsgathered) (Variables|Default|GetNObjectInLevel))
    (TimeManagement|PauseChrono)
    (bind _gi (CallFunction|GetGameInstance))
    (Default|GotoNextLevel _gi (Variables|Default|GetLevelTime))
    (else
      (Levels|ChangeMapMaterial ItemGathered)
      (Items|ApplyMovementEffect ItemGathered))))

(fn GetGameInstance
  (Utilities|IsValid (Variables|Default|GetGameInstance)
    (:Is%20Valid
      _)
    (:Is%20Not%20Valid
      (bind _asbp_game_instance (Utilities|Casting|CastToBP_GameInstance (Game|GetGameInstance)))
      (bind _output_get (Variables|Default|SetGameInstance _asbp_game_instance))))
  (return _output_get))

(fn ChangeMapMaterial
  (params (EffectType :type BP_ObjectTypes%20Enum :default "NewEnumerator0"))
  (bind _materialtype (Items|ConvertTypes EffectType))
  (bind _outactors (Actor|GetAllActorsOfClass "/Game/Tiles/BP_Tile.BP_Tile_C"))
  (for _array_element _outactors
    (Variables|/Game/Tiles/BP_Tile.BP_Tile_C|SetEffectType _array_element _materialtype)
    (Default|SetTileMaterial _array_element)))

(fn ConvertTypes
  (params (ObjectType :type BP_ObjectTypes%20Enum :default "NewEnumerator0"))
  (switch Utilities|FlowControl|Switch|SwitchonBP_ObjectTypes ObjectType
    (:NewEnumerator0
      (return "NewEnumerator5"))
    (:NewEnumerator1
      (return "NewEnumerator1"))
    (:NewEnumerator2
      (return "NewEnumerator2"))
    (:NewEnumerator3
      (return "NewEnumerator3"))
    (:NewEnumerator4
      (return "NewEnumerator4"))
    (:NewEnumerator5
      (return "NewEnumerator0"))))

(fn ApplyMovementEffect
  (params (ObjectType :type BP_ObjectTypes%20Enum :default "NewEnumerator0"))
  (bind _returnvalue (Game|GetPlayerCharacter 0))
  (bind _rotationratestandard (Variables|PlayerMovements|GetRotationRateStandard))
  (bind _maxwalkspeedstandard (Variables|PlayerMovements|GetMaxWalkSpeedStandard))
  (bind _brakingdecelerationstandard (Variables|PlayerMovements|GetBrakingDecelerationStandard))
  (bind _charactermovement (Variables|/Script/Engine.Character|GetCharacterMovement _returnvalue))
  (switch Utilities|FlowControl|Switch|SwitchonBP_ObjectTypes ObjectType
    (:NewEnumerator0
      (Variables|/Script/Engine.CharacterMovementComponent|SetRotationRate _charactermovement _rotationratestandard)
      (Variables|/Script/Engine.CharacterMovementComponent|SetMaxWalkSpeed _charactermovement (Variables|PlayerMovements|GetMaxWalkSpeedIncreased))
      (Variables|/Script/Engine.CharacterMovementComponent|SetBrakingDecelerationWalking _charactermovement _brakingdecelerationstandard))
    (:NewEnumerator1
      (Variables|/Script/Engine.CharacterMovementComponent|SetRotationRate _charactermovement _rotationratestandard)
      (Variables|/Script/Engine.CharacterMovementComponent|SetMaxWalkSpeed _charactermovement _maxwalkspeedstandard)
      (Variables|/Script/Engine.CharacterMovementComponent|SetBrakingDecelerationWalking _charactermovement _brakingdecelerationstandard))
    (:NewEnumerator2
      (Variables|/Script/Engine.CharacterMovementComponent|SetRotationRate _charactermovement (Variables|PlayerMovements|GetRotationRateReduced))
      (Variables|/Script/Engine.CharacterMovementComponent|SetMaxWalkSpeed _charactermovement (Variables|PlayerMovements|GetMaxWalkSpeedReduced))
      (Variables|/Script/Engine.CharacterMovementComponent|SetBrakingDecelerationWalking _charactermovement _brakingdecelerationstandard))
    (:NewEnumerator3
      (Variables|/Script/Engine.CharacterMovementComponent|SetRotationRate _charactermovement _rotationratestandard)
      (Variables|/Script/Engine.CharacterMovementComponent|SetMaxWalkSpeed _charactermovement _maxwalkspeedstandard)
      (Variables|/Script/Engine.CharacterMovementComponent|SetBrakingDecelerationWalking _charactermovement (Variables|PlayerMovements|GetBrakingDecelerationreduced)))
    (:NewEnumerator4
      (Variables|/Script/Engine.CharacterMovementComponent|SetRotationRate _charactermovement _rotationratestandard)
      (Variables|/Script/Engine.CharacterMovementComponent|SetMaxWalkSpeed _charactermovement _maxwalkspeedstandard)
      (Variables|/Script/Engine.CharacterMovementComponent|SetBrakingDecelerationWalking _charactermovement _brakingdecelerationstandard))
    (:NewEnumerator5
      (Variables|/Script/Engine.CharacterMovementComponent|SetRotationRate _charactermovement _rotationratestandard)
      (Variables|/Script/Engine.CharacterMovementComponent|SetMaxWalkSpeed _charactermovement _maxwalkspeedstandard)
      (Variables|/Script/Engine.CharacterMovementComponent|SetBrakingDecelerationWalking _charactermovement _brakingdecelerationstandard))))

(fn InitializeStartingPosition
  (Utilities|Array|Clear (Variables|MapAttributes|GetStartingPositions))
  (bind _outactors (Actor|GetAllActorsOfClass "/Script/Engine.TargetPoint"))
  (bind _output_get (Variables|MapAttributes|SetStartingPositions _outactors))
  (Utilities|Array|Shuffle _output_get))

(fn PickStartingPosition
  (params (Index :type Integer))
  (bind _startingpositions (Variables|MapAttributes|GetStartingPositions))
  (bind _returnvalue (Utilities|Array|Length _startingpositions))
  (if (== _returnvalue 0)
    (Levels|InitializeStartingPosition))
  (return (Utilities|Array|Get(acopy) (Variables|MapAttributes|GetStartingPositions) (Math|Integer|%(Integer) Index _returnvalue))))

(fn PlacePlayerandObjects
  (Levels|InitializeStartingPosition)
  (bind _output (Levels|PickStartingPosition))
  (Transformation|SetActorLocationAndRotation (Game|GetPlayerCharacter 0) (.location (Transformation|GetActorTransform _output)) (.rotation (Transformation|GetActorTransform _output)))
  (for _index (range 0 (- (Variables|Default|GetNObjectInLevel) 1))
    (bind _output_2 (Levels|PickStartingPosition (+ _index 1)))
    (Game|SpawnActorfromClass "/Game/objects/BP_Object.BP_Object_C" (Math|Transform|MakeTransform (.location (Transformation|GetActorTransform _output_2)) (.rotation (Transformation|GetActorTransform _output_2)) "1,1,1") "Undefined" 0 (Utilities|Enum|ByteToEnumBP_ObjectTypes (Math|Conversions|ToByte(Integer) (Math|Random|RandomIntegerinRange 0 (- (|GetNumEnumEntries) 2)))) 0)))